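; VR test actor that shows the battery percentage of a chosen WaveVR device on a text render.
; It starts with a default string, then rewrites the text with device name and level whenever the bound WaveVR battery status event fires and the reading is positive.
; A delayed Tick polls roughly once a second while the Checked flag is set, clearing it after the first non-negative reading.
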(event Custom|CustomEvent_0
  (bind _device (Variables|Default|Getdevice))
  (bind _returnvalue (Class|WaveVRBlueprintFunctionLibrary|GetDeviceBatteryPercentage _device))
  (if (> _returnvalue 0.0)
    (Rendering|Components|TextRender|SetText (Variables|Default|GetTextRender) (Utilities|Text|ToText(String) (Utilities|String|Append (Utilities|String|EnumtoString _device) ", battery: " (Utilities|String|ToString(Float) _returnvalue))))
    (Development|PrintString "battery update")))

(event EventBeginPlay
  (Rendering|Components|TextRender|SetText (Variables|Default|GetTextRender) (Variables|Default|Getdefault%20str))
  (EventDispatchers|BindEventtoWaveVRonBatteryStatusUpdate (Variables|Default|GetBatteryStatusEvent) (delegate Custom|CustomEvent_0)))

(event EventTick
  (params (DeltaSeconds :type Float%20%28single-precision%29))
  (bind _device (Variables|Default|Getdevice))
  (Utilities|FlowControl|Delay 1.0)
  (if (Variables|Default|Getchecked)
    (bind _returnvalue (Class|WaveVRBlueprintFunctionLibrary|GetDeviceBatteryPercentage _device))
    (if (>= _returnvalue 0.0)
      (Variables|Default|Setchecked false)
      (Rendering|Components|TextRender|SetText (Variables|Default|GetTextRender) (Utilities|Text|ToText(String) (Utilities|String|Append (Utilities|String|EnumtoString _device) ", battery: " (Utilities|String|ToString(Float) _returnvalue)))))))

(fn ConstructionScript)