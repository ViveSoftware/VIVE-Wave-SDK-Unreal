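; Test actor for WaveVR that shows headset and left/right controller battery levels and connection state on a batteryInfo widget.
; CheckAll runs CheckBattery per device on BeginPlay, on WaveVR battery status events, and about once a second through a Delay on Tick.
; Connected devices are read only while their cached valid flag is false.
; Disconnected devices or non-positive readings go to SetFailure, which zeroes the level and clears the connected flag.
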(event Custom|CustomEvent_0
  (CallFunction|CheckAll))

(event EventBeginPlay
  (EventDispatchers|BindEventtoWaveVRonBatteryStatusUpdate (Variables|Default|GetBatteryStatusEvent) (delegate Custom|CustomEvent_0))
  (bind _asbattery_info (Utilities|Casting|CastTobatteryInfo (UserInterface|GetUserWidgetObject (Variables|Default|GetWidget))))
  (Variables|Default|SetbatteryWidgetObj _asbattery_info)
  (CallFunction|CheckAll))

(event Collision|EventActorBeginOverlap
  (params (OtherActor :type Actor%20Object%20Reference)))

(event EventTick
  (params (DeltaSeconds :type Float%20%28single-precision%29))
  (Utilities|FlowControl|Delay 1.0)
  (CallFunction|CheckAll))

(fn ConstructionScript)

(fn CheckBattery
  (params (device :type EWVR_DeviceType%20Enum :default "DeviceType_Invalid"))
  (bind _batterywidgetobj (Variables|Default|GetbatteryWidgetObj))
  (bind _batterywidgetobj_2 (Variables|Default|GetbatteryWidgetObj))
  (bind _batterywidgetobj_3 (Variables|Default|GetbatteryWidgetObj))
  (bind _returnvalue (Class|WaveVRBlueprintFunctionLibrary|IsDeviceConnected device))
  (if _returnvalue
    (switch Utilities|FlowControl|Switch|SwitchonEWVR_DeviceType device
      (:DeviceType_HMD
        (if (not (Variables|Default|GetisHMDBatteryValid))
          (bind _returnvalue_2 (Class|WaveVRBlueprintFunctionLibrary|GetDeviceBatteryPercentage device :!label _label))
          (if (> _returnvalue_2 0.0)
            (switch Utilities|FlowControl|Switch|SwitchonEWVR_DeviceType device
              (:DeviceType_HMD
                (Variables|/Game/VRTestApp/BatteryStatus_Test/batteryInfo.batteryInfo_C|SetHMDBattery _batterywidgetobj _returnvalue_2)
                (Variables|/Game/VRTestApp/BatteryStatus_Test/batteryInfo.batteryInfo_C|SetisHMDConnected _batterywidgetobj true))
              (:DeviceType_Controller_Right
                (Variables|/Game/VRTestApp/BatteryStatus_Test/batteryInfo.batteryInfo_C|SetRightBattery _batterywidgetobj_2 _returnvalue_2)
                (Variables|/Game/VRTestApp/BatteryStatus_Test/batteryInfo.batteryInfo_C|SetisRightConnected _batterywidgetobj_2 true))
              (:DeviceType_Controller_Left
                (Variables|/Game/VRTestApp/BatteryStatus_Test/batteryInfo.batteryInfo_C|SetLeftBattery _batterywidgetobj_3 _returnvalue_2)
                (Variables|/Game/VRTestApp/BatteryStatus_Test/batteryInfo.batteryInfo_C|SetisLeftConnected _batterywidgetobj_3 true)))
            (return true)
            (else
              (CallFunction|SetFailure device :!label _label_2)
              (return false)))))
      (:DeviceType_Controller_Right
        (if (not (Variables|Default|GetisRightValid))
          (goto _label)))
      (:DeviceType_Controller_Left
        (if (not (Variables|Default|GetisLeftValid))
          (goto _label))))
    (else
      (goto _label_2))))

(fn CheckAll
  (Utilities|FlowControl|Sequence
    (:then_0
      (bind _valid (CallFunction|CheckBattery "DeviceType_HMD"))
      (Variables|Default|SetisHMDBatteryValid _valid))
    (:then_1
      (bind _valid_2 (CallFunction|CheckBattery "DeviceType_Controller_Right"))
      (Variables|Default|SetisRightValid _valid_2))
    (:then_2
      (bind _valid_3 (CallFunction|CheckBattery "DeviceType_Controller_Left"))
      (Variables|Default|SetisLeftValid _valid_3))))

(fn SetFailure
  (params (device :type EWVR_DeviceType%20Enum :default "DeviceType_Invalid"))
  (bind _batterywidgetobj (Variables|Default|GetbatteryWidgetObj))
  (bind _batterywidgetobj_2 (Variables|Default|GetbatteryWidgetObj))
  (bind _batterywidgetobj_3 (Variables|Default|GetbatteryWidgetObj))
  (switch Utilities|FlowControl|Switch|SwitchonEWVR_DeviceType device
    (:DeviceType_HMD
      (Variables|/Game/VRTestApp/BatteryStatus_Test/batteryInfo.batteryInfo_C|SetHMDBattery _batterywidgetobj_2 0.0)
      (Variables|/Game/VRTestApp/BatteryStatus_Test/batteryInfo.batteryInfo_C|SetisHMDConnected _batterywidgetobj_2 false))
    (:DeviceType_Controller_Right
      (Variables|/Game/VRTestApp/BatteryStatus_Test/batteryInfo.batteryInfo_C|SetRightBattery _batterywidgetobj_3 0.0)
      (Variables|/Game/VRTestApp/BatteryStatus_Test/batteryInfo.batteryInfo_C|SetisRightConnected _batterywidgetobj_3 false))
    (:DeviceType_Controller_Left
      (Variables|/Game/VRTestApp/BatteryStatus_Test/batteryInfo.batteryInfo_C|SetLeftBattery _batterywidgetobj 0.0)
      (Variables|/Game/VRTestApp/BatteryStatus_Test/batteryInfo.batteryInfo_C|SetisLeftConnected _batterywidgetobj false))))