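; BallActor01_Blueprint is a WaveVR HelloVR ball that changes material when pointed at and toggles 100 units along Y when selected.
; BeginPlay caches the WaveVR_Pawn, whose input-module hit results Tick tests by actor class, not instance.
; Controller modes color it red (right), blue (left) or green (untargeted), using trigger or touchpad presses to move it.
; Gaze mode selects by timeout, right touchpad or both, using delays and DoOnce gates.
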(event EventBeginPlay
  (Utilities|FlowControl|Sequence
    (:then_1
      (bind _outactors (Actor|GetAllActorsOfClass "/WaveVR/Blueprints/WaveVR_Pawn.WaveVR_Pawn_C"))
      (for _array_element _outactors
        (if (== (Utilities|GetClass _array_element) "/WaveVR/Blueprints/WaveVR_Pawn.WaveVR_Pawn_C")
          (Variables|Default|SetwaveVR_Pawn _array_element))))))

(event EventTick
  (params (DeltaSeconds :type Float%20%28single-precision%29))
  (bind _returnvalue (Transformation|GetActorLocation))
  (bind _returnvalue_2 (Transformation|GetActorLocation))
  (bind _returnvalue_3 (Transformation|GetActorLocation))
  (bind _wavevr_pawn (Variables|Default|GetwaveVR_Pawn))
  (bind _wavevr_pawn_2 (Variables|Default|GetwaveVR_Pawn))
  (bind _timetogaze (Variables|/WaveVR/Blueprints/WaveVR_Pawn.WaveVR_Pawn_C|GetTimeToGaze _wavevr_pawn_2))
  (bind _inputmodulemgr (Variables|/WaveVR/Blueprints/WaveVR_Pawn.WaveVR_Pawn_C|GetInputModuleMgr _wavevr_pawn))
  (bind _gazelasthitresult (Variables|/WaveVR/Blueprints/WaveVRInputModuleManager.WaveVRInputModuleManager_C|GetGazeLastHitResult _inputmodulemgr))
  (bind _hitactor (Collision|BreakHitResult _gazelasthitresult))
  (bind _returnvalue_4 (Utilities|GetClass _hitactor))
  (bind _returnvalue_5 (== _returnvalue_4 "ballActor01_Blueprint_C"))
  (bind _returnvalue_6 (Class|WaveVRInputFunctionLibrary|GetInteractionMode))
  (switch Utilities|FlowControl|Switch|SwitchonEWVR_InteractionMode _returnvalue_6
    (:InteractionMode_SystemDefault
      (bind _returnvalue_7 (Class|WaveVRBlueprintFunctionLibrary|GetFocusController :!label _label))
      (Utilities|FlowControl|Sequence
        (:then_0
          (if (Utilities|Enum|Equal(Enum) _returnvalue_7 "DeviceType_Controller_Right")
            ;[1 1 1] controllerRight
            (if (== (Utilities|GetClass (.HitActor (Collision|BreakHitResult (Variables|/WaveVR/Blueprints/WaveVRInputModuleManager.WaveVRInputModuleManager_C|GetLastHitResult_Right (Variables|/WaveVR/Blueprints/WaveVR_Pawn.WaveVR_Pawn_C|GetInputModuleMgr (Variables|Default|GetwaveVR_Pawn)))))) "ballActor01_Blueprint_C")
              (Rendering|Material|SetMaterial (Variables|Debug|GetStaticMeshComponent) 0 "/Game/HelloVR/Texture/ball_Red.ball_red")
              (Utilities|FlowControl|Sequence
                (:then_0
                  (bind _returnvalue_8 (Class|WaveVRInputFunctionLibrary|IsInputButtonPressed "DeviceType_Controller_Right" "Touchpad"))
                  (if (Math|Boolean|ORBoolean _returnvalue_8 (stale _returnvalue_9) (stale _returnvalue_10))
                    (Utilities|FlowControl|DoOnce false :!label _label_2
                      (:Completed
                        (Utilities|FlowControl|Sequence
                          (:then_0
                            (Utilities|FlowControl|Delay 0.2)
                            (goto _label_2 Reset))
                          (:then_1
                            (if (Variables|Default|Getmove_controllerRClicked)
                              (Transformation|SetActorLocation (- _returnvalue_2 "0,100.000000, 0") false false)
                              (Variables|Default|Setmove_controllerRClicked false)
                              (else
                                (Transformation|SetActorLocation (+ _returnvalue_2 "0,100.000000, 0") false false)
                                (Variables|Default|Setmove_controllerRClicked true)))))))))
                (:then_1
                  (bind _returnvalue_9 (Class|WaveVRInputFunctionLibrary|IsInputButtonPressed "DeviceType_Controller_Right" "Digital_Trigger")))
                (:then_2
                  (bind _returnvalue_10 (Class|WaveVRInputFunctionLibrary|IsInputButtonPressed "DeviceType_Controller_Right" "Trigger"))))
              (else
                (Rendering|Material|SetMaterial (Variables|Debug|GetStaticMeshComponent) 0 "/Game/HelloVR/Texture/ball_green.ball_green")))))
        (:then_1
          (if (Utilities|Enum|Equal(Enum) _returnvalue_7 "DeviceType_Controller_Left")
            (Utilities|FlowControl|Sequence
              (:then_0
                ;[1 1 1] controllerLeft
                (if (== (Utilities|GetClass (.HitActor (Collision|BreakHitResult (Variables|/WaveVR/Blueprints/WaveVRInputModuleManager.WaveVRInputModuleManager_C|GetLastHitResult_Left (Variables|/WaveVR/Blueprints/WaveVR_Pawn.WaveVR_Pawn_C|GetInputModuleMgr (Variables|Default|GetwaveVR_Pawn)))))) "ballActor01_Blueprint_C")
                  (Rendering|Material|SetMaterial (Variables|Debug|GetStaticMeshComponent) 0 "/Game/HelloVR/Texture/ball_blue.ball_blue")
                  (Utilities|FlowControl|Sequence
                    (:then_0
                      (bind _returnvalue_11 (Class|WaveVRInputFunctionLibrary|IsInputButtonPressed "DeviceType_Controller_Left" "Touchpad"))
                      (if (Math|Boolean|ORBoolean _returnvalue_11 (stale _returnvalue_12) (stale _returnvalue_13))
                        (Utilities|FlowControl|DoOnce false :!label _label_3
                          (:Completed
                            (Utilities|FlowControl|Sequence
                              (:then_0
                                (Utilities|FlowControl|Delay 0.2)
                                (goto _label_3 Reset))
                              (:then_1
                                (if (Variables|Default|Getmove_controllerLClicked)
                                  (Transformation|SetActorLocation (+ _returnvalue_3 "0,100.000000, 0") false false)
                                  (Variables|Default|Setmove_controllerLClicked false)
                                  (else
                                    (Transformation|SetActorLocation (- _returnvalue_3 "0,100.000000, 0") false false)
                                    (Variables|Default|Setmove_controllerLClicked true)))))))))
                    (:then_1
                      (bind _returnvalue_12 (Class|WaveVRInputFunctionLibrary|IsInputButtonPressed "DeviceType_Controller_Left" "Trigger")))
                    (:then_2
                      (bind _returnvalue_13 (Class|WaveVRInputFunctionLibrary|IsInputButtonPressed "DeviceType_Controller_Left" "Digital_Trigger"))))
                  (else
                    (Rendering|Material|SetMaterial (Variables|Debug|GetStaticMeshComponent) 0 "/Game/HelloVR/Texture/ball_green.ball_green")))))))))
    (:InteractionMode_Gaze
      ;[1 1 1] Gaze
      (if _returnvalue_5
        (Rendering|Material|SetMaterial (Variables|Debug|GetStaticMeshComponent) 0 0)
        (bind _returnvalue_14 (Class|WaveVRInputFunctionLibrary|GetGazeTriggerType))
        (switch Utilities|FlowControl|Switch|SwitchonEWVR_GazeTriggerType _returnvalue_14
          (:GazeTriggerType_Timeout
            ;;[1 1 1] GazeTimeOut
            (Utilities|FlowControl|Delay _timetogaze)
            (if _returnvalue_5
              (if (Variables|Default|Getmove_gazeClicked) :!label _label_4
                (Transformation|SetActorLocation (- _returnvalue "0,100.000000, 0") false false)
                (Variables|Default|Setmove_gazeClicked false)
                (else
                  (Transformation|SetActorLocation (+ _returnvalue "0,100.000000, 0") false false)
                  (Variables|Default|Setmove_gazeClicked true)))))
          (:GazeTriggerType_Button
            ;;[1 1 1] GazeButton
            (bind _returnvalue_15 (Class|WaveVRInputFunctionLibrary|IsInputButtonPressed "DeviceType_Controller_Right" "Touchpad" :!label _label_5))
            (if _returnvalue_15
              (Utilities|FlowControl|DoOnce false :!label _label_6
                (:Completed
                  (Utilities|FlowControl|Sequence
                    (:then_0
                      (goto _label_4))
                    (:then_1
                      (goto _label_7 Reset))
                    (:then_2
                      (Utilities|FlowControl|Delay 0.2)
                      (goto _label_6 Reset)))))))
          (:GazeTriggerType_TimeoutButton
            (Utilities|FlowControl|Sequence
              (:then_0
                (goto _label_5))
              (:then_1
                ;;[1 1 1] GazeTimeout(ButtonTimeout)
                (Utilities|FlowControl|DoOnce false :!label _label_7
                  (:Completed
                    (Utilities|FlowControl|RetriggerableDelay _timetogaze)
                    (if _returnvalue_5
                      (Utilities|FlowControl|Sequence
                        (:then_0
                          (goto _label_4))
                        (:then_1
                          (goto _label_7 Reset))))))))))
        (else
          (Rendering|Material|SetMaterial (Variables|Debug|GetStaticMeshComponent) 0 0)
          (goto _label_7 Reset))))
    (:InteractionMode_Controller
      (goto _label))))

(fn ConstructionScript)